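; DisplayScore_BP is a score display that shows a number on a text render, apparently for a bowling game given its pin and roll naming.
; SetNewScore writes a given value straight to the text, while AddtoScore adds pins to a running CurrentRoll total and displays it.
; When that total reaches one or more, it sends a flash message to every entry in Lights, using IsFlashing to avoid repeats until the total drops below one.
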(event EventSetNewScore
  (params (NewScore :type Integer))
  (Rendering|Components|TextRender|SetText (Variables|Default|GetTextRender) (Utilities|Text|ToText(Integer) NewScore)))

(event EventAddtoScore
  (params (PinsToAdd :type Integer))
  (bind _output_get (Variables|Default|SetCurrentRoll (+ PinsToAdd (Variables|Default|GetCurrentRoll))))
  (Rendering|Components|TextRender|SetText (Variables|Default|GetTextRender) (Utilities|Text|ToText(Integer) _output_get))
  (if (< _output_get 1)
    (Variables|Default|SetisFlashing false)
    (elif (not (Variables|Default|GetisFlashing))
      (Variables|Default|SetisFlashing true)
      (for _array_element (Variables|Default|GetLights)
        (Class|ScoreInterface|FlashLights(Message) _array_element)))))

(fn ConstructionScript)