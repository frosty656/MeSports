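; A grabbable physics dodgeball for VR motion controllers that launches itself away when a pawn comes near.
; Pickup disables physics and attaches it to the controller, and Drop reverses both.
; Each tick it sphere-checks for pawns: the first hit teleports it to a fixed height, then hits during a five-second window apply spin and a fixed-direction impulse.
; Tick re-enables physics every frame, even after a pickup.
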(event EventPickup
  (params (AttachTo :type Scene%20Component%20Object%20Reference))
  (Physics|SetSimulatePhysics (Variables|Debug|GetStaticMeshComponent) false)
  (Transformation|AttachComponentToComponent (VehicleSound|GetRootComponent) AttachTo "None" "KeepWorld" "KeepWorld" "KeepWorld" false))

(event EventDrop
  (Physics|SetSimulatePhysics (Variables|Debug|GetStaticMeshComponent) true)
  (Transformation|DetachFromActor "KeepWorld" "KeepWorld" "KeepWorld"))

(event EventTick
  (params (DeltaSeconds :type Float%20%28single-precision%29))
  (bind _staticmeshcomponent (Variables|Debug|GetStaticMeshComponent))
  (bind _staticmeshcomponent_2 (Variables|Debug|GetStaticMeshComponent))
  (bind _returnvalue (Transformation|GetWorldLocation _staticmeshcomponent))
  (bind (_x _y) (Math|Vector|BreakVector _returnvalue))
  (bind _outactors (Collision|SphereOverlapActors (Transformation|GetWorldLocation (Variables|Debug|GetStaticMeshComponent)) 1e+02 (Utilities|Array|MakeArray "ObjectTypeQuery3") 0))
  (if (> (Utilities|Array|Length _outactors) 0)
    (Physics|SetSimulatePhysics (Variables|Debug|GetStaticMeshComponent) true)
    (if (Variables|Default|GethasMovedUp)
      (Class|PrimitiveComponent|SetPhysicsAngularVelocityinDegrees _staticmeshcomponent_2 (Math|Vector|MakeVector 45.0 (Math|Random|RandomFloatinRange 2e+01 6e+01) 45.0) false "None")
      (Physics|AddImpulse _staticmeshcomponent_2 "500.000000,0.000000,100.000000" "None" true)
      (else
        (Variables|Default|SethasMovedUp true)
        (Transformation|SetWorldLocation (Variables|Debug|GetStaticMeshComponent) (Math|Vector|MakeVector _x _y 3.6e+02) false false)
        (Utilities|FlowControl|Delay 5.0)
        (Variables|Default|SethasMovedUp false)))
    (else
      (Physics|SetSimulatePhysics (Variables|Debug|GetStaticMeshComponent) true))))

(fn ConstructionScript)